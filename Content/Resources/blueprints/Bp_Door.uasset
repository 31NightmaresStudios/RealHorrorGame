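; Interactive door that the first-person player opens and closes with E while standing inside its trigger box.
; Box overlap enables input on the actor and shows an Interact_interface prompt widget, and leaving disables input and removes it.
; A FlipFlop alternates playing and reversing the AbrirPuerta timeline, which lerps the door's yaw between closed and open angles, with a 2D sound for each direction.
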(event OnComponentBeginOverlap(Box)
  (params (OverlappedComponent :type Primitive%20Component%20Object%20Reference) (OtherActor :type Actor%20Object%20Reference) (OtherComp :type Primitive%20Component%20Object%20Reference) (OtherBodyIndex :type Integer) (bFromSweep :type Boolean) (SweepResult :type Hit%20Result%20Structure%20%28by%20ref%29))
  ;[1 1 1] ¿Ha entrado en la caja?
  ;[1 1 1] El jugador entró en la caja
  (Utilities|Casting|CastToBP_FirstPersonCharacter OtherActor)
  (Input|EnableInput (Game|GetPlayerController 0))
  ;[1 1 1] Mostrar interface
  (bind _returnvalue (UserInterface|CreateWidget "/Game/interfaces/Interact_interface.Interact_interface_C"))
  (UserInterface|Viewport|AddtoViewport _returnvalue 0))

(event OnComponentEndOverlap(Box)
  (params (OverlappedComponent :type Primitive%20Component%20Object%20Reference) (OtherActor :type Actor%20Object%20Reference) (OtherComp :type Primitive%20Component%20Object%20Reference) (OtherBodyIndex :type Integer))
  (Utilities|Casting|CastToBP_FirstPersonCharacter OtherActor)
  (Input|DisableInput (Game|GetPlayerController 0))
  ;[1 1 1] Ocultar interface
  (Widget|RemovefromParent (stale OnComponentBeginOverlap(Box) _returnvalue)))

(event Input|KeyboardEvents|E
  (params (Key :type Key%20Structure :default "None"))
  ;[1 1 1] Accion
  (:Pressed
    (Utilities|FlowControl|FlipFlop
      (:A
        (Audio|PlaySound2D "/Game/Resources/sounds/opening-the-front-door-210347.opening-the-front-door-210347" 1.0 1.0 0.0 0 0)
        (bind _animpuerta (Timeline|Abrir%20Puerta Play)
          (:Update
            (Transformation|SetRelativeRotation (Variables|Default|GetDoor) (Math|Rotator|MakeRotator 0.0 0.0 (Math|Float|Lerp (Variables|Default|GetPuerta%20Cerrada) (Variables|Default|GetPuerta%20Abierta) _animpuerta)) false false))))
      (:B
        (Audio|PlaySound2D "/Game/Resources/sounds/Puerta_closing.Puerta_closing" 1.0 1.0 0.0 0 0)
        (Timeline|Abrir%20Puerta Reverse)))))

(fn ConstructionScript)